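; CellSignal_Cylinder is an overlap zone that sets the player's cell signal level.
; When the player's TopDownCharacter starts overlapping it, the zone passes its CellSignalLevel to SetCellSignal.
; When the overlap ends, it sets the signal to one below that level rather than restoring the previous value.
; Other actors are ignored by comparing against player character 0.
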(event `self.ReceiveActorBeginOverlap`
  (params (OtherActor :type "Actor Object Reference"))
  (bind _astop_down_character (cast `/Game/Blueprints/TopDownCharacter` (`GameplayStatics.GetPlayerCharacter` 0)))
  (if (== OtherActor _astop_down_character)
    (`/Game/Blueprints/TopDownCharacter.Set_CellSignal` _astop_down_character (`self.CellSignal_Level`))))

(event `self.ReceiveActorEndOverlap`
  (params (OtherActor :type "Actor Object Reference"))
  (bind _astop_down_character (cast `/Game/Blueprints/TopDownCharacter` (`GameplayStatics.GetPlayerCharacter` 0)))
  (if (== OtherActor _astop_down_character)
    (`/Game/Blueprints/TopDownCharacter.Set_CellSignal` _astop_down_character (- (`self.CellSignal_Level`) 1))))

(fn `UserConstructionScript`)