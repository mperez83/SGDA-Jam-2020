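; CellSignal_Manager is an actor for a drifting cell signal circle that exists for a limited time.
; On BeginPlay it picks a random yaw and destroys itself after the VTimeAlive delay.
; Tick steps it along its forward vector by a fixed, frame-rate-dependent amount.
; A helper to randomly offset inner circles in X and Y exists, but its calls are unconnected and marked TODO.
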(event `self.ReceiveBeginPlay`
  ;[1 1 1] Set Rotation to determine directional movement. Then Start delay timer for how long it will last.
  (`self.K2_SetActorRotation` (`KismetMathLibrary.MakeRotator` 0.0 0.0 (`KismetMathLibrary.Conv_IntToDouble` (`KismetMathLibrary.RandomInteger` 360))) true)
  (`KismetSystemLibrary.Delay` (`self.vTimeAlive`))
  (`self.K2_DestroyActor`))

(event `self.ReceiveTick`
  (params (DeltaSeconds :type "Float (single-precision)"))
  ;[1 1 1] Move the circle in the relative forward direction
  (`self.K2_SetActorRelativeLocation` (+ (`self.K2_GetActorLocation`) (`self.GetActorForwardVector`))))

(fn `InnitializeInnerCircle`
  (params (currentCircle :type "/Game/Blueprints/CellSignal_Cylinder Object Reference"))
  (`self.K2_SetActorRelativeLocation` currentCircle (`KismetMathLibrary.MakeVector` (`KismetMathLibrary.Conv_IntToDouble` (`KismetMathLibrary.RandomIntegerInRange` -200 200)) (`KismetMathLibrary.Conv_IntToDouble` (`KismetMathLibrary.RandomIntegerInRange` -200 200))) false false))

(fn `UserConstructionScript`)