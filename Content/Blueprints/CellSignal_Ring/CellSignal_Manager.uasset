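; CellSignal_Manager is a short-lived actor for a cell signal ring that drifts across the level in a random direction.
; BeginPlay picks a random yaw and destroys the actor after VTimeAlive, while Tick steps it forward without delta-time scaling.
; SetInnerRingValues gives four child CellSignal_Cylinder circles incrementing signal levels from Count, but is not called here.
; Random offsetting of inner circles is an unfinished TODO whose calls never run.
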(event `self.ReceiveBeginPlay`
  ;[1 1 1] Set Rotation to determine directional movement. Then Start delay timer for how long it will last.
  (`self.K2_SetActorRotation` (`KismetMathLibrary.MakeRotator` 0.0 0.0 (`KismetMathLibrary.Conv_IntToDouble` (`KismetMathLibrary.RandomInteger` 360))) true)
  (`KismetSystemLibrary.Delay` (`self.vTimeAlive`))
  (`self.K2_DestroyActor`))

(event `self.ReceiveTick`
  (params (DeltaSeconds :type "Float (single-precision)"))
  ;[1 1 1] Move the circle in the relative forward direction
  (`self.K2_SetActorRelativeLocation` (+ (`self.K2_GetActorLocation`) (`self.GetActorForwardVector`))))

(fn `InnitializeInnerCircle`
  (params (currentCircle :type "/Game/Blueprints/CellSignal_Ring/CellSignal_Cylinder Object Reference"))
  (`self.K2_SetActorRelativeLocation` currentCircle (`KismetMathLibrary.MakeVector` (`KismetMathLibrary.Conv_IntToDouble` (`KismetMathLibrary.RandomIntegerInRange` -200 200)) (`KismetMathLibrary.Conv_IntToDouble` (`KismetMathLibrary.RandomIntegerInRange` -200 200))) false false))

(fn `Set_InnerRingValues`
  (locals (count :type Integer :default 1))
  (bind _ascell_signal_cylinder (cast `/Game/Blueprints/CellSignal_Ring/CellSignal_Cylinder` (`ChildActorComponent.ChildActor` (`self.Circle_1`))))
  (bind _output_get (set `/Game/Blueprints/CellSignal_Ring/CellSignal_Cylinder.CellSignal_Level` (`local.count`) _ascell_signal_cylinder))
  (bind _result (`/Engine/EditorBlueprintResources/StandardMacros.IncrementInt` _output_get)
    (:`  `
      (bind _ascell_signal_cylinder_2 (cast `/Game/Blueprints/CellSignal_Ring/CellSignal_Cylinder` (`ChildActorComponent.ChildActor` (`self.Circle_2`))))
      (bind _output_get_2 (set `/Game/Blueprints/CellSignal_Ring/CellSignal_Cylinder.CellSignal_Level` _result _ascell_signal_cylinder_2))
      (bind _result_2 (`/Engine/EditorBlueprintResources/StandardMacros.IncrementInt` _output_get_2)
        (:`  `
          (bind _ascell_signal_cylinder_3 (cast `/Game/Blueprints/CellSignal_Ring/CellSignal_Cylinder` (`ChildActorComponent.ChildActor` (`self.Circle_3`))))
          (bind _output_get_3 (set `/Game/Blueprints/CellSignal_Ring/CellSignal_Cylinder.CellSignal_Level` _result_2 _ascell_signal_cylinder_3))
          (bind _result_3 (`/Engine/EditorBlueprintResources/StandardMacros.IncrementInt` _output_get_3)
            (:`  `
              (bind _ascell_signal_cylinder_4 (cast `/Game/Blueprints/CellSignal_Ring/CellSignal_Cylinder` (`ChildActorComponent.ChildActor` (`self.Circle_4`))))
              (set `/Game/Blueprints/CellSignal_Ring/CellSignal_Cylinder.CellSignal_Level` _result_3 _ascell_signal_cylinder_4))))))))

(fn `UserConstructionScript`)