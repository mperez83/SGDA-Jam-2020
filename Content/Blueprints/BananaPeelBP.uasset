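; Banana peel hazard actor that makes an overlapping TopDownCharacter slip and go flying.
; If the character is not already ragdolled, it calls Yeet along the normalized velocity with an upward component, flagged to lose the phone.
; It then plays a slip sound and destroys itself, so each peel triggers once.
; BeginPlay caches the player character, but the overlap logic does not use that reference.
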(event `self.ReceiveBeginPlay`
  (bind _astop_down_character (cast `/Game/Blueprints/TopDownCharacter` (`GameplayStatics.GetPlayerCharacter` 0))))

(event `self.ReceiveActorBeginOverlap`
  (params (OtherActor :type "Actor Object Reference"))
  (bind _astop_down_character (cast `/Game/Blueprints/TopDownCharacter` OtherActor))
  (if (not (`/Game/Blueprints/TopDownCharacter.Ragdolled` _astop_down_character))
    (bind (_returnvalue_x _returnvalue_y) (`KismetMathLibrary.BreakVector` (`KismetMathLibrary.Normal` (`self.GetVelocity` _astop_down_character))))
    (`/Game/Blueprints/TopDownCharacter.Yeet` _astop_down_character (`KismetMathLibrary.MakeVector` _returnvalue_x _returnvalue_y 0.75) 40.0 true)
    (`GameplayStatics.PlaySoundAtLocation` "/Game/Audio/Sounds/Banana_Slip.Banana_Slip" (`self.K2_GetActorLocation`) (struct) 2.0 1.0 0.0 null null null)
    (`self.K2_DestroyActor`)))

(fn `UserConstructionScript`)