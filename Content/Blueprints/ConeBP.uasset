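; ConeBP is a traffic-cone-style physics prop that gets knocked away when the top-down player character runs into it.
; On overlap with a TopDownCharacter, it applies a strong impulse to the Cone component, pointing away from the character horizontally with a fixed upward lift.
; It also plays a kick sound at its location.
; A player reference is cached on BeginPlay but not used by the impact logic.
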(event `self.ReceiveBeginPlay`
  (bind _astop_down_character (cast `/Game/Blueprints/TopDownCharacter` (`GameplayStatics.GetPlayerCharacter` 0))))

(event `self.ReceiveActorBeginOverlap`
  (params (OtherActor :type "Actor Object Reference"))
  (bind (_returnvalue_x _returnvalue_y) (`KismetMathLibrary.BreakVector` (* (`KismetMathLibrary.Normal` (- (`self.K2_GetActorLocation`) (`self.K2_GetActorLocation` OtherActor))) 10000.0)))
  (cast `/Game/Blueprints/TopDownCharacter` OtherActor)
  (`PrimitiveComponent.AddImpulse` (`self.Cone`) (`KismetMathLibrary.MakeVector` _returnvalue_x _returnvalue_y 8000.0) "None" false)
  (`GameplayStatics.PlaySoundAtLocation` "/Game/Audio/Sounds/Cone_Kick_Cue.Cone_Kick_Cue" (`self.K2_GetActorLocation`) (struct) 1.0 1.0 0.0 null null null))

(fn `UserConstructionScript`)