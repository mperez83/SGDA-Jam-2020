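; MainMenuLogoBP is a main menu logo Blueprint that gently wobbles its mesh.
; Each Tick advances an angle at a frame-rate independent rate, wrapping it past a full turn.
; Sine waves of that angle at different frequencies drive small roll, pitch and yaw offsets on the Mesh's relative rotation.
; Pitch and yaw share the same wave, while roll swings slower and wider.
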(event `self.ReceiveTick`
  (params (DeltaSeconds :type "Float (single-precision)"))
  (bind _output_get (set `self.MainDeg` (+ (`self.MainDeg`) (* DeltaSeconds 60.0))))
  (if (> _output_get 360.0)
    (set `self.MainDeg` (- (`self.MainDeg`) 360.0)))
  (`SceneComponent.K2_SetRelativeRotation` (`self.Mesh`) (`KismetMathLibrary.MakeRotator` (* (`KismetMathLibrary.DegSin` (* (`self.MainDeg`) 2.0)) 5.0) (* (`KismetMathLibrary.DegSin` (* (`self.MainDeg`) 3.0)) 2.0) (* (`KismetMathLibrary.DegSin` (* (`self.MainDeg`) 3.0)) 2.0)) false false))

(fn `UserConstructionScript`)