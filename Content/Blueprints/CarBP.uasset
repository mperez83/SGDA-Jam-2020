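; CarBP is a cart actor that rides along the spline of a referenced track actor.
; On BeginPlay, if active, it plays a timeline at a rate set by its duration, from a configurable start offset.
; Each update maps the timeline alpha to distance along the spline and sets world location and rotation from that point.
; A hit from the TopDownCharacter only prints a debug message.
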(event `self.ReceiveBeginPlay`
  (if (`self.ActiveCart`)
    (`self.MoveCart`)))

(event `self.ReceiveHit`
  (params (MyComp :type "PrimitiveComponent Object Reference") (Other :type "Actor Object Reference") (OtherComp :type "PrimitiveComponent Object Reference") (bSelfMoved :type Boolean) (HitLocation :type "Vector Structure") (HitNormal :type "Vector Structure") (NormalImpulse :type "Vector Structure") (Hit :type "HitResult Structure (by ref)"))
  (cast `/Game/Blueprints/TopDownCharacter` Other)
  (`KismetSystemLibrary.PrintString` "ow"))

(event `MoveCart`
  (bind _returnvalue (`KismetMathLibrary.Lerp` 0.0 (`SplineComponent.GetSplineLength` (`/Game/Blueprints/CarTrack.UsefulSpline` (`self.TrackRef`))) (`self.Alpha`)))
  (`TimelineComponent.SetPlayRate` (`self.CartMover`) (/ 1.0 (`self.Duration`)))
  (`TimelineComponent.SetNewTime` (`self.CartMover`) (`self.CartStartOffset`))
  (bind (_direction _alpha) (`Timeline|CartMover`)
    (:`Update`
      (set `self.Alpha` _alpha)
      (`self.K2_SetActorLocationAndRotation` (`SplineComponent.GetLocationAtDistanceAlongSpline` (`/Game/Blueprints/CarTrack.UsefulSpline` (`self.TrackRef`)) _returnvalue "World") (`SplineComponent.GetRotationAtDistanceAlongSpline` (`/Game/Blueprints/CarTrack.UsefulSpline` (`self.TrackRef`)) _returnvalue "World")))))

(fn `UserConstructionScript`)