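; Phone store pickup actor that gives the TopDownCharacter a phone when they walk into it.
; On overlap it checks whether the character already has a phone, and if not calls PickUpPhone and plays a launch-pad sound at its location.
; EnableHitbox and DisableHitbox toggle the trigger area's visibility along with the box's overlap event generation.
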(event `self.ReceiveActorBeginOverlap`
  (params (OtherActor :type "Actor Object Reference"))
  (bind _astop_down_character (cast `/Game/Blueprints/TopDownCharacter` OtherActor))
  (bind _newparam (`/Game/Blueprints/TopDownCharacter.Get_IfHasPhone` _astop_down_character))
  (if (not _newparam)
    (`/Game/Blueprints/TopDownCharacter.PickUpPhone` _astop_down_character)
    (`GameplayStatics.PlaySoundAtLocation` "/Game/Audio/Sounds/LaunchPad_Launch.LaunchPad_Launch" (`self.K2_GetActorLocation`) (struct) 1.0 1.0 0.0 null null null)))

(fn `DisableHitbox`
  (`SceneComponent.SetVisibility` (`self.TriggerArea`) false false)
  (set `PrimitiveComponent.bGenerateOverlapEvents` false (`self.Box`)))

(fn `EnableHitbox`
  (`SceneComponent.SetVisibility` (`self.TriggerArea`) true false)
  (set `PrimitiveComponent.bGenerateOverlapEvents` true (`self.Box`)))

(fn `UserConstructionScript`)