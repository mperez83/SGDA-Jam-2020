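; A pedestrian NPC that travels along a referenced spline track and knocks away the player character on contact.
; When active, one timeline moves it along the spline from a start offset over a set duration, while another bobs its mesh.
; Overlapping a non-ragdolled TopDownCharacter yeets them upward and away, making them lose their phone, with a punch sound and "Pow" sprite.
; It then briefly throws a fit, bobbing faster and higher before calming down.
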(event `self.ReceiveBeginPlay`
  (if (`self.ActiveCart`)
    (`self.MoveCart`)
    (`self.Bob Event`)))

(event `self.ReceiveActorBeginOverlap`
  (params (OtherActor :type "Actor Object Reference"))
  (bind _astop_down_character (cast `/Game/Blueprints/TopDownCharacter` OtherActor))
  (if (not (`/Game/Blueprints/TopDownCharacter.Ragdolled` _astop_down_character))
    (bind (_returnvalue_x _returnvalue_y) (`KismetMathLibrary.BreakVector` (`KismetMathLibrary.Normal` (- (`self.K2_GetActorLocation` _astop_down_character) (`self.K2_GetActorLocation`)))))
    (`/Game/Blueprints/TopDownCharacter.Yeet` _astop_down_character (`KismetMathLibrary.MakeVector` _returnvalue_x _returnvalue_y 1.0) 25.0 true)
    (`GameplayStatics.PlaySoundAtLocation` "/Game/Audio/Sounds/Pedestrian_Punch.Pedestrian_Punch" (`SceneComponent.K2_GetComponentLocation` (`self.Mesh`)) (struct) 1.0 1.0 0.0 null null null)
    (bind _returnvalue (`|SpawnActorFromClass` "/Game/Blueprints/ComicFXBP.ComicFXBP_C" (`KismetMathLibrary.Conv_VectorToTransform` (`KismetMathLibrary.VLerp` (`SceneComponent.K2_GetComponentLocation` (`/Game/Blueprints/TopDownCharacter.ActualMesh` _astop_down_character)) (`SceneComponent.K2_GetComponentLocation` (`self.Capsule`)) 0.5)) "Undefined" "OverrideRootScale" null null))
    (`PaperSpriteComponent.SetSprite` (`/Game/Blueprints/ComicFXBP.PaperSprite` _returnvalue) "/Game/Graphics/2D_Assets/Pow_Effect_Sprite.Pow_Effect_Sprite")
    (`self.Have A Fit`)))

(event `MoveCart`
  (bind _returnvalue (`KismetMathLibrary.Lerp` 0.0 (`SplineComponent.GetSplineLength` (`/Game/Blueprints/CarTrack.UsefulSpline` (`self.TrackRef`))) (`self.Alpha`)))
  (`TimelineComponent.SetPlayRate` (`self.CartMover`) (/ 1.0 (`self.Duration`)))
  (`TimelineComponent.SetNewTime` (`self.CartMover`) (`self.CartStartOffset`))
  (bind (_direction _alpha) (`Timeline|CartMover`)
    (:`Update`
      (set `self.Alpha` _alpha)
      (`self.K2_SetActorLocationAndRotation` (`SplineComponent.GetLocationAtDistanceAlongSpline` (`/Game/Blueprints/CarTrack.UsefulSpline` (`self.TrackRef`)) _returnvalue "World") (`SplineComponent.GetRotationAtDistanceAlongSpline` (`/Game/Blueprints/CarTrack.UsefulSpline` (`self.TrackRef`)) _returnvalue "World") true))))

(event `Bob Event`
  (`TimelineComponent.SetPlayRate` (`self.Bobber`) 5.0)
  (bind (_direction _z_val) (`Timeline|Bobber`)
    (:`Update`
      (`SceneComponent.K2_SetRelativeLocation` (`self.MeshPivot`) (`KismetMathLibrary.MakeVector` 0.0 0.0 (* _z_val (`self.BobHeight`))) false false))))

(event `Have A Fit`
  (if (not (`self.Angry`))
    (set `self.Angry` true)
    (`TimelineComponent.SetPlayRate` (`self.Bobber`) 15.0)
    (set `self.BobHeight` 40.0)
    (`GameplayStatics.PlaySoundAtLocation` "/Game/Audio/Sounds/LaunchPad_Launch.LaunchPad_Launch" (`SceneComponent.K2_GetComponentLocation` (`self.Capsule`)) (struct) 1.0 1.0 0.0 null null null)
    (`KismetSystemLibrary.Delay` 2.0)
    (`TimelineComponent.SetPlayRate` (`self.Bobber`) 5.0)
    (set `self.BobHeight` 10.0)
    (set `self.Angry` false)))

(fn `UserConstructionScript`)