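; Physical phone actor that the player's TopDownCharacter picks up by touching it.
; BeginPlay caches the player character, then enables pickup after a short delay.
; Once enabled, Tick polls the trigger box for overlap with the player rather than using overlap events, then calls PickUpPhone on the character and destroys the actor.
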(event `self.ReceiveBeginPlay`
  (bind _astop_down_character (cast `/Game/Blueprints/TopDownCharacter` (`GameplayStatics.GetPlayerCharacter` 0)))
  (set `self.Player` _astop_down_character)
  (`KismetSystemLibrary.Delay` 2.0)
  (set `self.CanBePickedUp` true))

(event `self.ReceiveTick`
  (params (DeltaSeconds :type "Float (single-precision)"))
  (bind _player (`self.Player`))
  (if (`self.CanBePickedUp`)
    (if (`PrimitiveComponent.IsOverlappingActor` (`self.PickupTriggerBox`) _player)
      (`/Game/Blueprints/TopDownCharacter.PickUpPhone` _player)
      (`self.K2_DestroyActor`))))

(fn `UserConstructionScript`)